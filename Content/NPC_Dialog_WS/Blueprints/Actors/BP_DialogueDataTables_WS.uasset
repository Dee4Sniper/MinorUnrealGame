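; Actor that fills dialogue and choice-response arrays from data tables for an NPC dialogue system.
; On BeginPlay it loops over every row name in DialogueDataTable and adds each found row to DialogueEntries.
; The two optional choice tables are copied into Choice01Response and Choice02Response only from that loop's Row Not Found branch, so they stay unread when every dialogue row resolves.
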(event EventBeginPlay
  (bind _dialogue_data_table (Variables|Default|GetDialogue%20Data%20Table))
  ;[0.2135 0.2135 0.2135] Set dialogue based on data table
  (|CallParentFunction)
  (bind _outrownames (DataTable|GetDataTableRowNames _dialogue_data_table))
  (for _array_element _outrownames
    (bind _returnvalue (Utilities|GetDataTableRow _dialogue_data_table _array_element)
      (:then
        (Utilities|Array|Add (Variables|Default|GetDialogueEntries) _returnvalue))
      (:RowNotFound
        ;[0.2135 0.2135 0.2135] Set choice 01 response based on data table
        (bind _choice_01_data_table (Variables|Default|GetChoice%2001%20Data%20Table)
          (:then
            (bind _outrownames_2 (DataTable|GetDataTableRowNames _choice_01_data_table))
            (for _array_element_2 _outrownames_2
              (bind _returnvalue_2 (Utilities|GetDataTableRow _choice_01_data_table _array_element_2)
                (:then
                  (Utilities|Array|Add (Variables|Default|GetChoice%2001%20Response) _returnvalue_2)))))
          (:else
            _))
        ;[0.2135 0.2135 0.2135] Set choice 02 response based on data table
        (bind _choice_02_data_table (Variables|Default|GetChoice%2002%20Data%20Table)
          (:then
            (bind _outrownames_3 (DataTable|GetDataTableRowNames _choice_02_data_table))
            (for _array_element_3 _outrownames_3
              (bind _returnvalue_3 (Utilities|GetDataTableRow _choice_02_data_table _array_element_3)
                (:then
                  (Utilities|Array|Add (Variables|Default|GetChoice%2002%20Response) _returnvalue_3)))))
          (:else))))))

(event Collision|EventActorBeginOverlap
  (params (OtherActor :type Actor%20Object%20Reference)))

(event EventTick
  (params (DeltaSeconds :type Float%20%28single-precision%29)))

(fn ConstructionScript
  (|CallParentFunction))