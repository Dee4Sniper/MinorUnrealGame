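; NPC character that can offer dialogue to the player and shows a talk widget while the player character overlaps its sphere.
; On BeginPlay, dialogue-enabled NPCs spawn a separate dialogue actor with entries, choices and a parent reference.
; A valid dialogue table loads rows into those arrays and selects BP_DialogueDataTables_WS; otherwise BP_Dialogue_WS receives the existing arrays.
; Random wandering and fixed-route AIMoveTo chains are present but unconnected.
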(event OnComponentBeginOverlap(Sphere)
  (params (OverlappedComponent :type Primitive%20Component%20Object%20Reference) (OtherActor :type Actor%20Object%20Reference) (OtherComp :type Primitive%20Component%20Object%20Reference) (OtherBodyIndex :type Integer) (bFromSweep :type Boolean) (SweepResult :type Hit%20Result%20Structure%20%28by%20ref%29))
  ;[0.2135 0.2135 0.2135] Show and hide speech widget above character
  (CallFunction|ToggleTalkNotificationWidget OtherActor true))

(event OnComponentEndOverlap(Sphere)
  (params (OverlappedComponent :type Primitive%20Component%20Object%20Reference) (OtherActor :type Actor%20Object%20Reference) (OtherComp :type Primitive%20Component%20Object%20Reference) (OtherBodyIndex :type Integer))
  ;[0.2135 0.2135 0.2135] Show and hide speech widget above character
  (CallFunction|ToggleTalkNotificationWidget OtherActor false))

(event EventBeginPlay
  ;[0.2135 0.2135 0.2135] Spawn dialogue actor if character can speak to player
  (CallFunction|SpawnDialogueActor))

(fn ConstructionScript)

(fn SpawnDialogueActor
  (if (Variables|Dialogue|GetContains%20Dialogue)
    (Utilities|IsValid (Variables|DataTables|GetDialogue%20Data%20Table)
      (:Is%20Valid
        ;[0.2135 0.2135 0.2135] Initialize data table
        (bind _dialogue_data_table (Variables|DataTables|GetDialogue%20Data%20Table)
          (:then
            (bind _outrownames (DataTable|GetDataTableRowNames _dialogue_data_table))
            (for _array_element _outrownames
              (bind _returnvalue (Utilities|GetDataTableRow _dialogue_data_table _array_element)
                (:then
                  (Utilities|Array|Add (Variables|Dialogue|GetDialogue%20Entries) _returnvalue)))))
          (:else
            _))
        (bind _choice_01_data_table (Variables|DataTables|GetChoice%2001%20Data%20Table)
          (:then
            (bind _outrownames_2 (DataTable|GetDataTableRowNames _choice_01_data_table))
            (for _array_element_2 _outrownames_2
              (bind _returnvalue_2 (Utilities|GetDataTableRow _choice_01_data_table _array_element_2)
                (:then
                  (Utilities|Array|Add (Variables|Choices|GetChoice%2001%20Response) _returnvalue_2)))))
          (:else
            _))
        (bind _choice_02_data_table (Variables|DataTables|GetChoice%2002%20Data%20Table)
          (:then
            (bind _outrownames_3 (DataTable|GetDataTableRowNames _choice_02_data_table))
            (for _array_element_3 _outrownames_3
              (bind _returnvalue_3 (Utilities|GetDataTableRow _choice_02_data_table _array_element_3)
                (:then
                  (Utilities|Array|Add (Variables|Choices|GetChoice%2002%20Response) _returnvalue_3)))))
          (:else
            _))
        (Game|SpawnActorfromClass "/Game/NPC_Dialog_WS/Blueprints/Actors/BP_DialogueDataTables_WS.BP_DialogueDataTables_WS_C" (Transformation|GetActorTransform) "Undefined" 0 (Variables|Dialogue|GetDialogue%20Entries) false (Variables|Choices|GetContains%20Choice) (Variables|Choices|GetChoices%20Loop) (Variables|Choices|GetChoice%2001) (Variables|Choices|GetChoice%2002) (Variables|Choices|GetChoice%2001%20Response) (Variables|Choices|GetChoice%2002%20Response) (Variables|Dialogue|GetNPC%20Rotates) self 0))
      (:Is%20Not%20Valid
        ;[0.2135 0.2135 0.2135] Initialize Default
        (Game|SpawnActorfromClass "/Game/NPC_Dialog_WS/Blueprints/Actors/BP_Dialogue_WS.BP_Dialogue_WS_C" (Transformation|GetActorTransform) "Undefined" 0 (Variables|Dialogue|GetDialogue%20Entries) (Variables|Dialogue|GetDisable%20Text%20Animation?) (Variables|Choices|GetContains%20Choice) (Variables|Choices|GetChoices%20Loop) (Variables|Choices|GetChoice%2001) (Variables|Choices|GetChoice%2002) (Variables|Choices|GetChoice%2001%20Response) (Variables|Choices|GetChoice%2002%20Response) (Variables|Dialogue|GetNPC%20Rotates) self 0)))))

(fn ToggleTalkNotificationWidget
  (params (Target :type Actor%20Object%20Reference) (bNewVisibility :type Boolean))
  (if (Variables|Dialogue|GetContains%20Dialogue)
    (Utilities|Casting|CastToAS_BP_ThirdPersonCharacter (Game|GetInstigator Target))
    (Rendering|SetVisibility (Variables|Default|GetTalk%20Widget) bNewVisibility false)))